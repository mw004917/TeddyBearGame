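; BP_Train is a train actor that travels along the spline of a referenced track, starting on BeginPlay.
; AllAboard plays a timeline at a rate of one thirtieth and maps its track value to distance along the spline, setting the world location each update.
; When the timeline finishes, it calls Arrived on its parent manager.
; The node that would align rotation to the spline is unconnected, so only location changes.
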(event Custom|AllAboard
  (bind _trackref (Variables|Default|GetTrackRef))
  (bind _spline (Variables|/Game/TrainBP/TrainTracks.TrainTracks_C|GetSpline _trackref))
  (Variables|Default|SetNewPlayRate (/ 1.0 3e+01))
  (Components|Timeline|SetPlayRate (Variables|Default|GetTimeline_0) (Variables|Default|GetNewPlayRate))
  (bind _newtrack_0 (Timeline|Timeline_0 Play)
    (:Update
      (Transformation|SetActorLocation (Spline|GetLocationatDistanceAlongSpline _spline (* _newtrack_0 (Spline|GetSplineLength _spline)) "World") false false))
    (:Finished
      (Default|Arrived (Variables|Default|GetParentManager)))))

(event EventBeginPlay
  (CallFunction|AllAboard))

(fn ConstructionScript)