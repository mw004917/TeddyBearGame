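; Train carriage actor that carries a random resource container along the spline of its referenced track.
; On BeginPlay it spawns a scaled-down container of one of six item types at its arrow, attaches it, then calls AllAboard.
; AllAboard plays a slowed timeline that maps its track value to distance along the spline, updating location only.
; Arrived stops the timeline; the node aligning rotation to the spline is unconnected.
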(event Custom|Arrived
  (bind _trackref (Variables|Default|GetTrackRef))
  (bind _spline (Variables|/Game/TrainBP/TrainTracks.TrainTracks_C|GetSpline _trackref))
  (bind _newtrack_0 (Timeline|Timeline_0 Stop)
    (:Update
      (Transformation|SetActorLocation (Spline|GetLocationatDistanceAlongSpline _spline (* _newtrack_0 (Spline|GetSplineLength _spline)) "World") false false))))

(event Custom|AllAboard
  (bind _trackref (Variables|Default|GetTrackRef))
  (bind _spline (Variables|/Game/TrainBP/TrainTracks.TrainTracks_C|GetSpline _trackref))
  (Variables|Default|SetPlayRate (/ 1.0 3e+01))
  (Components|Timeline|SetPlayRate (Variables|Default|GetTimeline_0) (Variables|Default|GetPlayRate))
  (bind _newtrack_0 (Timeline|Timeline_0 Play)
    (:Update
      (Transformation|SetActorLocation (Spline|GetLocationatDistanceAlongSpline _spline (* _newtrack_0 (Spline|GetSplineLength _spline)) "World") false false))))

(event EventBeginPlay
  (bind _returnvalue (Game|SpawnActorfromClass "/Game/ThirdPersonBP/TomsStuff/ResourceContainerBASE.ResourceContainerBASE_C" (Math|Transform|MakeTransform (Transformation|GetWorldLocation (Variables|Default|GetArrow)) "0.000000,90.000000, 0" "0.250000,0.250000,0.250000") "AlwaysSpawn" 0 (Utilities|Enum|ByteToEnumWhichItemToSpawn (Math|Conversions|ToByte(Integer) (Math|Random|RandomIntegerinRange 0 5))) 0))
  (Transformation|AttachActorToActor _returnvalue self "None" "KeepWorld" "KeepWorld" "KeepWorld" true)
  (CallFunction|AllAboard))

(fn ConstructionScript)