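; BP_Carriage is a train carriage that carries a randomly chosen resource container along a spline track.
; On BeginPlay it spawns the container at its arrow, attaches it, then calls AllAboard to play a slowed timeline.
; The timeline's output scales the TrackRef spline's length to set the carriage's location and rotation.
; Separate events reverse the timeline, stop it on arrival, or destroy the attached container.
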(event Custom|Arrived
  (bind _trackref (Variables|Default|GetTrackRef))
  (bind _spline (Variables|/Game/TeddyWars/Blueprints/Tom/Train/TrainTracks.TrainTracks_C|GetSpline _trackref))
  (bind _newtrack_0 (Timeline|Timeline_0 Stop)
    (:Update
      (Transformation|SetActorLocation (Spline|GetLocationatDistanceAlongSpline _spline (* _newtrack_0 (Spline|GetSplineLength _spline)) "World") false false)
      (Transformation|SetActorRotation (Spline|GetRotationatDistanceAlongSpline (Variables|/Game/TeddyWars/Blueprints/Tom/Train/TrainTracks.TrainTracks_C|GetSpline (Variables|Default|GetTrackRef)) (* _newtrack_0 (Spline|GetSplineLength _spline)) "World")))))

(event Custom|AllAboard
  (bind _trackref (Variables|Default|GetTrackRef))
  (bind _spline (Variables|/Game/TeddyWars/Blueprints/Tom/Train/TrainTracks.TrainTracks_C|GetSpline _trackref))
  (Variables|Default|SetPlayRate (/ 1.0 15.0))
  (Components|Timeline|SetPlayRate (Variables|Default|GetTimeline_0) (Variables|Default|GetPlayRate))
  (bind _newtrack_0 (Timeline|Timeline_0 Play)
    (:Update
      (Transformation|SetActorLocation (Spline|GetLocationatDistanceAlongSpline _spline (* _newtrack_0 (Spline|GetSplineLength _spline)) "World") false false)
      (Transformation|SetActorRotation (Spline|GetRotationatDistanceAlongSpline (Variables|/Game/TeddyWars/Blueprints/Tom/Train/TrainTracks.TrainTracks_C|GetSpline (Variables|Default|GetTrackRef)) (* _newtrack_0 (Spline|GetSplineLength _spline)) "World")))))

(event Custom|Reverse
  (bind _trackref (Variables|Default|GetTrackRef))
  (bind _spline (Variables|/Game/TeddyWars/Blueprints/Tom/Train/TrainTracks.TrainTracks_C|GetSpline _trackref))
  (bind _newtrack_0 (Timeline|Timeline_0 Reverse)
    (:Update
      (Transformation|SetActorLocation (Spline|GetLocationatDistanceAlongSpline _spline (* _newtrack_0 (Spline|GetSplineLength _spline)) "World") false false)
      (Transformation|SetActorRotation (Spline|GetRotationatDistanceAlongSpline (Variables|/Game/TeddyWars/Blueprints/Tom/Train/TrainTracks.TrainTracks_C|GetSpline (Variables|Default|GetTrackRef)) (* _newtrack_0 (Spline|GetSplineLength _spline)) "World")))))

(event Custom|DeleteChild
  (Actor|DestroyActor (Variables|Default|GetChild)))

(event EventBeginPlay
  (bind _returnvalue (Game|SpawnActorfromClass "/Game/TeddyWars/Blueprints/Tom/ResourceContainer/ResourceContainerBASE.ResourceContainerBASE_C" (Math|Transform|MakeTransform (Transformation|GetWorldLocation (Variables|Default|GetArrow)) "0.000000,270.000000, 0" "0.500000,0.500000,0.500000") "AlwaysSpawn" 0 (Utilities|Enum|ByteToEnumWhichItemToSpawn (Math|Conversions|ToByte(Integer) (Math|Random|RandomIntegerinRange 3 5))) 0))
  (Variables|Default|SetChild _returnvalue)
  (Transformation|AttachActorToActor (Variables|Default|GetChild) self "None" "KeepWorld" "KeepWorld" "KeepWorld" true)
  (CallFunction|AllAboard))

(fn ConstructionScript)