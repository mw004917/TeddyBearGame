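; Game mode for Teddy Wars that ends the match when a team's base dies.
; On BeginPlay it caches the tagged GameCam, binds to the death event of every Base's Health and creates an additional local player.
; The death handler uses the base's TeamID to send a true or false game-over message to the first player controller, then pauses the game and sets a queryable game-over flag.
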(event EventBeginPlay
  ;[1 1 1] Cache Camera
  (bind _outactors (Actor|GetAllActorswithTag "Camera"))
  (bind _asgame_cam (Utilities|Casting|CastToGameCam (Utilities|Array|Get(acopy) _outactors)))
  (Variables|Default|SetCamera _asgame_cam)
  (bind _outactors_2 (Actor|GetAllActorsOfClass "/Game/TeddyWars/Blueprints/Steve/Base/Base.Base_C"))
  (for _array_element _outactors_2
    (EventDispatchers|BindEventtoDeathEvent (Variables|/Game/TeddyWars/Blueprints/Steve/Base/Base.Base_C|GetHealth _array_element) (EventDispatchers|CreateEvent :!event GMTeddyAutoGenFunc)))
  (Class|GameplayStatics|CreatePlayer -1))

(fn ConstructionScript)

(fn GMTeddyAutoGenFunc
  (params (Actor :type Actor%20Object%20Reference))
  (bind _asbase (Utilities|Casting|CastToBase Actor))
  (switch int (Variables|/Game/TeddyWars/Blueprints/Steve/Base/Base.Base_C|GetTeamID _asbase)
    (:0
      (Class|IPCP|Gameover(Message) (Game|GetPlayerController 0) false))
    (:1
      (Class|IPCP|Gameover(Message) (Game|GetPlayerController 0) true)))
  (Game|SetGamePaused true)
  (Variables|Default|SetIsGameOver true))

(fn GetIsGameOver
  (return (Variables|Default|GetIsGameOver)))